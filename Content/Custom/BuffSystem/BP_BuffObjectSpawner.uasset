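; BP_BuffObjectSpawner is a spawner actor that scatters random buff objects around its location.
; BeginPlay spawns an initial batch, then Tick runs a countdown timer that spawns another every few seconds, with no cap or cleanup.
; SpawnBuff takes a class picked at random from the Buffs array and spawns it at a random XY within a square area around the actor, at a fixed world height.
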(event `self.ReceiveBeginPlay`
  (set `self.SpawnTImer` 3.0)
  (for _ (range 6)
    (`self.SpawnBuff` (`KismetArrayLibrary.Array_Random` (`self.Buffs`)))))

(event `self.ReceiveTick`
  (params (DeltaSeconds :type "Float (single-precision)"))
  (bind _output_get (set `self.SpawnTImer` (- (`self.SpawnTImer`) DeltaSeconds)))
  (if (<= _output_get 0.0)
    (`self.SpawnBuff` (`KismetArrayLibrary.Array_Random` (`self.Buffs`)))
    (set `self.SpawnTImer` 3.0)))

(fn `SpawnBuff`
  (params (NewParam :type "/Game/Custom/BuffSystem/BP_BuffDebuffBase Class Reference"))
  (`|SpawnActorFromClass` NewParam (`KismetMathLibrary.Conv_VectorToTransform` (`KismetMathLibrary.MakeVector` (.x (`KismetMathLibrary.RandomPointInBoundingBox` (`self.K2_GetActorLocation`) (1000.0 1000.0 0.0))) (.y (`KismetMathLibrary.RandomPointInBoundingBox` (`self.K2_GetActorLocation`) (1000.0 1000.0 0.0))) -500.0)) "Undefined" "MultiplyWithRoot" null null))

(fn `UserConstructionScript`)