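; Base actor for a player buff or debuff effect, limited by duration and usage count.
; StartEffect registers it with the BP_UI widget, then for players controlled by MyPlayerController stores the target, sets lifespan and initializes usages.
; ReduceUsages computes Amount minus remaining usages and destroys the actor at zero or below.
; EndPlay calls EndEffect, which removes the buff class from the affected player.
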(event `Start Effect`
  (params (AffectedPlayer :type "/Game/Custom/BP_Player1 Object Reference"))
  ;[1 1 1] Set UI HUD
  (bind _foundwidgets (`WidgetBlueprintLibrary.GetAllWidgetsOfClass` "/Game/Custom/BP_UI.BP_UI_C"))
  (`/Game/Custom/BP_UI.AddBuff` (`|GetArrayItem` _foundwidgets) AffectedPlayer self)
  ;[1 1 1] Setup buff duration and usages
  (`/Engine/EditorBlueprintResources/StandardMacros.IsValid` AffectedPlayer
    (:`Is Valid`
      (cast `/Game/Custom/MyPlayerController` (`Pawn.GetController` AffectedPlayer))
      (set `self.AffectedPlayer` AffectedPlayer)
      (`self.SetLifeSpan` (`self.BuffDuration`))
      (set `self.BuffUsagesLeft` (`self.BuffUsages`)))))

(event `self.ReceiveEndPlay`
  (params (EndPlayReason :type "EEndPlayReason Enum" :default "Destroyed"))
  (bind _affectedplayer (`self.AffectedPlayer`))
  ;[1 1 1] On destroy (call end effect)
  (`/Engine/EditorBlueprintResources/StandardMacros.IsValid` _affectedplayer
    (:`Is Valid`
      (`self.End Effect` _affectedplayer))))

(event `End Effect`
  (params (AffectedPlayer :type "/Game/Custom/BP_Player1 Object Reference"))
  ;[1 1 1] End effect
  (`/Game/Custom/BP_Player1.Try Remove Buff` AffectedPlayer (`GameplayStatics.GetObjectClass` self)))

(fn `ReduceUsages`
  (params (Amount :type Integer))
  (bind _output_get (set `self.BuffUsagesLeft` (- Amount (`self.BuffUsagesLeft`))))
  (if (<= _output_get 0)
    (`self.K2_DestroyActor`)))

(fn `UserConstructionScript`)