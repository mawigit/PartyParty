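; Debuff effect in the custom buff system that applies weakness to an affected player by changing their BaseStrength vector.
; On start, it calls the parent logic, checks that the player is valid, removes the opposing strength buff if HasBuff reports true, then overrides BaseStrength.
; On end, it sets BaseStrength to hardcoded values rather than a saved original, then calls the parent logic.
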(event `self.Start Effect`
  (params (AffectedPlayer :type "/Game/Custom/BP_Player1 Object Reference"))
  ;[1 1 1] Buff logic
  (`parent.Start Effect` AffectedPlayer)
  (`/Engine/EditorBlueprintResources/StandardMacros.IsValid` AffectedPlayer
    (:`Is Valid`
      (bind _hasbuff (`/Game/Custom/BP_Player1.Has Buff` AffectedPlayer null))
      (if _hasbuff
        (`/Game/Custom/BP_Player1.Try Remove Buff` AffectedPlayer "/Game/Custom/BuffSystem/Effects/BP_BuffStrengthEffect.BP_BuffStrengthEffect_C"))
      (set `/Game/Custom/BP_Player1.BaseStrength` (500.0 2000.0 0.0) AffectedPlayer))))

(event `self.End Effect`
  (params (AffectedPlayer :type "/Game/Custom/BP_Player1 Object Reference"))
  ;[1 1 1] End buff
  (set `/Game/Custom/BP_Player1.BaseStrength` (1000.0 1000.0 0.0) AffectedPlayer)
  (`parent.End Effect` AffectedPlayer))

(fn `UserConstructionScript`
  (`parent.UserConstructionScript`))