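; BP_DebuffSlowEffect is a buff-system effect that slows the affected player's walk speed.
; On start it runs the parent logic, removes any active speed buff if the player has a buff, then lowers the CharacterMovement max walk speed.
; On end it sets walk speed back to a hardcoded default, rather than a saved previous value, before running the parent end logic.
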(event `self.Start Effect`
  (params (AffectedPlayer :type "/Game/Custom/BP_Player1 Object Reference"))
  ;[1 1 1] Apply buff
  (`parent.Start Effect` AffectedPlayer)
  (`/Engine/EditorBlueprintResources/StandardMacros.IsValid` AffectedPlayer
    (:`Is Valid`
      (bind _hasbuff (`/Game/Custom/BP_Player1.Has Buff` AffectedPlayer null))
      (if _hasbuff
        (`/Game/Custom/BP_Player1.Try Remove Buff` AffectedPlayer "/Game/Custom/BuffSystem/Effects/BP_BuffSpeedEffect.BP_BuffSpeedEffect_C"))
      (set `CharacterMovementComponent.MaxWalkSpeed` 250.0 (`Character.CharacterMovement` AffectedPlayer)))))

(event `self.End Effect`
  (params (AffectedPlayer :type "/Game/Custom/BP_Player1 Object Reference"))
  ;[1 1 1] End buff
  (set `CharacterMovementComponent.MaxWalkSpeed` 500.0 (`Character.CharacterMovement` AffectedPlayer))
  (`parent.End Effect` AffectedPlayer))

(fn `UserConstructionScript`
  (`parent.UserConstructionScript`))