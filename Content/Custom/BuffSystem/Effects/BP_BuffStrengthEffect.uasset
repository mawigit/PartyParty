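; BP_BuffStrengthEffect is a buff effect actor that doubles the player's BaseStrength for as long as it exists.
; Shortly after BeginPlay, it casts its attach parent actor to BP_Player1 and overwrites the X and Y of BaseStrength with boosted values.
; EndPlay writes back hardcoded default values rather than restoring the previously stored strength.
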(event `self.ReceiveBeginPlay`
  (`parent.ReceiveBeginPlay`)
  (`KismetSystemLibrary.Delay` 0.2)
  (bind _asbp_player_1 (cast `/Game/Custom/BP_Player1` (`self.GetAttachParentActor`)))
  (set `/Game/Custom/BP_Player1.BaseStrength` (2000.0 2000.0 0.0) _asbp_player_1))

(event `self.ReceiveEndPlay`
  (params (EndPlayReason :type "EEndPlayReason Enum" :default "Destroyed"))
  (bind _asbp_player_1 (cast `/Game/Custom/BP_Player1` (`self.GetAttachParentActor`)))
  (set `/Game/Custom/BP_Player1.BaseStrength` (1000.0 1000.0 0.0) _asbp_player_1))

(fn `UserConstructionScript`
  (`parent.UserConstructionScript`))