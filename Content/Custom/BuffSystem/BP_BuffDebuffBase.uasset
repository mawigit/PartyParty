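; BP_BuffDebuffBase is a base pickup actor that grants a buff or debuff when a BP_Player1 overlaps it.
; A buff is applied to the collecting player via TryAddBuff, and the pickup is destroyed only if that succeeds.
; A debuff is sent to every other BP_Player1 and always consumes the pickup.
; The construction script sets a random lifespan, so uncollected pickups expire on their own.
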(event `self.ReceiveActorBeginOverlap`
  (params (OtherActor :type "Actor Object Reference"))
  (bind _asbp_player_1 (cast `/Game/Custom/BP_Player1` OtherActor))
  (bind _success (`self.AddBuff` _asbp_player_1))
  (if _success
    (`self.K2_DestroyActor`)))

(fn `AddBuff`
  (params (PickupPlayer :type "/Game/Custom/BP_Player1 Object Reference"))
  (returns (Success :type Boolean))
  (if (`self.IsDebuff`)
    (bind _outactors (`GameplayStatics.GetAllActorsOfClass` "/Game/Custom/BP_Player1.BP_Player1_C"))
    (for _array_element _outactors
      (if (not (== _array_element PickupPlayer))
        (`/Game/Custom/BP_Player1.Try Add Buff` _array_element (`self.BuffEffect`))))
    (return true)
    (else
      (bind _buffapplied (`/Game/Custom/BP_Player1.Try Add Buff` PickupPlayer (`self.BuffEffect`)))
      (return _buffapplied))))

(fn `UserConstructionScript`
  (`self.SetLifeSpan` (`KismetMathLibrary.RandomFloatInRange` 7.5 15.0)))