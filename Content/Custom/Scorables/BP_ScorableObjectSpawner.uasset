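; BP_ScorableObjectSpawner populates the level with scorable objects at BeginPlay, based on the SuddenDeath flag loaded from the SaveGameHS save slot.
; In sudden death it spawns a single golden ball; otherwise it spawns nine objects, each a random pick from ScorableObjectTypes.
; SpawnScorableObject places each one at a random point in a flat box centred on the spawner.
; Nothing spawns if the save fails to cast.
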(event `self.ReceiveBeginPlay`
  (bind _returnvalue (`GameplayStatics.LoadGameFromSlot` "SaveFile"))
  (bind _assave_game_hs (cast `/Game/UI/SaveGameHS` _returnvalue))
  (set `self.SuddenDeath` (`/Game/UI/SaveGameHS.SuddenDeath` _assave_game_hs))
  (if (`self.SuddenDeath`)
    (for _ (range 1)
      (`self.SpawnScorableObject`))
    (else
      (for _ (range 9)
        (`self.SpawnScorableObject`)))))

(fn `SpawnScorableObject`
  (bind _output_get (set `self.NewLocation` (`KismetMathLibrary.RandomPointInBoundingBox` (`self.K2_GetActorLocation`) (800.0 800.0 0.0))))
  (if (`self.SuddenDeath`)
    (bind _returnvalue (`KismetMathLibrary.Conv_VectorToTransform` _output_get))
    (`|SpawnActorFromClass` "/Game/Custom/Scorables/BP_ScorableGoldenBall.BP_ScorableGoldenBall_C" _returnvalue "Undefined" "MultiplyWithRoot" null null)
    (else
      (`|SpawnActorFromClass` (`KismetArrayLibrary.Array_Random` (`self.ScorableObjectTypes`)) _returnvalue "Undefined" "MultiplyWithRoot" null null))))

(fn `UserConstructionScript`)