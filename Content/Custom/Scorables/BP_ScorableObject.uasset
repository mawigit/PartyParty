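; BP_ScorableObject is a physics-simulated object that players touch to claim and score points with when it reaches a teleport zone.
; Overlapping a BP_Player1 records that character as last toucher and copies its mesh material onto the body.
; Overlapping a TeleportZone destroys it, plays a sound, has BP_ScorableObjectSpawner spawn a replacement with an explosion effect there, and awards Score to the last toucher.
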(event `self.ReceiveBeginPlay`
  (bind _scorableobjectbody (`self.ScorableObjectBody`))
  (`PrimitiveComponent.SetSimulatePhysics` _scorableobjectbody true)
  (`PrimitiveComponent.SetEnableGravity` _scorableobjectbody true))

(event `self.ReceiveActorBeginOverlap`
  (params (OtherActor :type "Actor Object Reference"))
  (bind _lasttouchedcharacter (`self.LastTouchedCharacter`))
  (cast `/Game/Custom/TeleportZone` OtherActor
    (:`then`
      (`self.K2_DestroyActor`)
      (`GameplayStatics.PlaySound2D` "/Game/SFX/345297__scrampunk__itemize.345297__scrampunk__itemize" 1.0 1.0 0.0 null null)
      (bind _returnvalue (`GameplayStatics.GetActorOfClass` "/Game/Custom/Scorables/BP_ScorableObjectSpawner.BP_ScorableObjectSpawner_C"))
      (`/Game/Custom/Scorables/BP_ScorableObjectSpawner.SpawnScorableObject` _returnvalue)
      (`GameplayStatics.SpawnEmitterAtLocation` "/Game/StarterContent/Particles/P_Explosion.P_Explosion" (`/Game/Custom/Scorables/BP_ScorableObjectSpawner.NewLocation` _returnvalue))
      (`/Engine/EditorBlueprintResources/StandardMacros.IsValid` _lasttouchedcharacter
        (:`Is Valid`
          (`/Game/Custom/BP_Player1.Add Score` _lasttouchedcharacter (`self.Score`))
          (set `self.LastTouchedCharacter` null) ; Setting last touched character to null
        )))
    (:`CastFailed`
      (bind _asbp_player_1 (cast `/Game/Custom/BP_Player1` OtherActor))
      (bind _output_get (set `self.LastTouchedCharacter` _asbp_player_1))
      (`PrimitiveComponent.SetMaterial` (`self.ScorableObjectBody`) 0 (`PrimitiveComponent.GetMaterial` (`Character.Mesh` _output_get) 0)))))

(fn `UserConstructionScript`)