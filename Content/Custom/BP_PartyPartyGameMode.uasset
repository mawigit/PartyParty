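; Game mode for a timed local multiplayer round that tracks top scores.
; BeginPlay reads the player count from SaveGameHS, creates local players, possesses a BP_Player1 spawned at each PlayerStart and initializes the BP_UI HUD.
; Tick counts down one minute, then GameFinished shows the winner widget, frees the mouse for UI and saves qualifying scores into gold, silver and bronze slots, shifting lower ranks down.
; CheckWinCondition and StopAllPlayerInput are unfinished stubs.
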(event `self.ReceiveBeginPlay`
  (bind _returnvalue (`GameplayStatics.GetPlayerController` 0))
  ;[0.1146 0.216 1] GetPlayerCount
  (set `self.Time` 60.0)
  (bind _returnvalue_2 (`GameplayStatics.LoadGameFromSlot` "SaveFile"))
  (bind _assave_game_hs (cast `/Game/UI/SaveGameHS` _returnvalue_2))
  (set `self.CurrentPlayerCount` (`/Game/UI/SaveGameHS.PlayerCount` _assave_game_hs))
  ;[1 0.3369 0.8202] Apply HUD
  (bind _returnvalue_3 (`|CreateWidget` "/Game/Custom/BP_UI.BP_UI_C"))
  (bind _output_get (set `self.UI` _returnvalue_3))
  (`UserWidget.AddToViewport` (`self.UI`) 0)
  (`UserWidget.AddToViewport` _output_get 0)
  ;[0.2142 1 0.3261] Create Player If Needed
  (bind _outactors (`GameplayStatics.GetAllActorsOfClass` "/Script/Engine.PlayerStart"))
  (for (_array_element _array_index) _outactors
    (if (< _array_index (`self.CurrentPlayerCount`))
      (bind _output_get_2 (set `self.Array Index` _array_index))
      (bind _returnvalue_4 (`GameplayStatics.CreatePlayer` _output_get_2))
      ;[1 0.1935 0.9256] Not Player 1
      (if (> (`self.Array Index`) 0)
        (`EnhancedInputSubsystemInterface.AddMappingContext` (pcsubsystem `EnhancedInputLocalPlayerSubsystem` _returnvalue_4) "/Game/ThirdPerson/Input/IMC_Default.IMC_Default" 0 (struct))
        (bind _returnvalue_5 (`self.GetTransform` _array_element))
        (bind _returnvalue_6 (`|SpawnActorFromClass` "/Game/Custom/BP_Player1.BP_Player1_C" _returnvalue_5 "Undefined" "MultiplyWithRoot" null null))
        (`Controller.Possess` (`GameplayStatics.GetPlayerController` (`self.Array Index`)) _returnvalue_6)
        (else
          ;[1 0.1935 0.9256] Player 1
          (`EnhancedInputSubsystemInterface.AddMappingContext` (pcsubsystem `EnhancedInputLocalPlayerSubsystem` _returnvalue) "/Game/ThirdPerson/Input/IMC_Default.IMC_Default" 0 (struct))
          (bind _returnvalue_7 (`|SpawnActorFromClass` "/Game/Custom/BP_Player1.BP_Player1_C" _returnvalue_5 "Undefined" "MultiplyWithRoot" null null))
          (`Controller.Possess` _returnvalue _returnvalue_7)))))
  ;[1 0.8252 0.04752] HUD
  (`/Game/Custom/BP_UI.InitPlayers` (`self.UI`) (`self.CurrentPlayerCount`)))

(event `GameFinished`
  (bind _returnvalue (`GameplayStatics.GetPlayerController` 0))
  ;[1 0.8252 0.04752] HUD
  (set `self.Finished` true)
  (bind _topscore (`/Game/Custom/BP_UI.DisplayWinnerWidget` (`self.UI`) (`self.CurrentPlayerCount`)))
  (`self.TryStoreHighScore` _topscore)
  (`WidgetBlueprintLibrary.SetInputMode_UIOnlyEx` _returnvalue null "LockOnCapture")
  (set `PlayerController.bEnableClickEvents` true _returnvalue)
  (set `PlayerController.bShowMouseCursor` true _returnvalue))

(event `self.ReceiveTick`
  (params (DeltaSeconds :type "Float (single-precision)"))
  (if (not (`self.Finished`))
    (`self.Timer`)
    (bind _over (`self.IsGameOver`))
    (if _over
      (`self.GameFinished`)
      (else
        ;[1 0.8252 0.04752] HUD
        (`/Game/Custom/BP_UI.UpdateTimer` (`self.UI`) (`self.Time`))))))

(event `Timer`
  ;[1 0.343 0.3729] Timer
  (set `self.Time` (- (`self.Time`) (`GameplayStatics.GetWorldDeltaSeconds`))))

(fn `CheckWinCondition`)

(fn `IsGameOver`
  (returns (over :type Boolean))
  (if (> (`self.Time`) 0.0)
    (return false)
    (else
      (return true))))

(fn `SaveNewBronzeScore`
  (params (SaveGameHS :type "/Game/UI/SaveGameHS Object Reference") (NewTopScore :type Integer))
  (set `/Game/UI/SaveGameHS.BronzeScore` NewTopScore SaveGameHS)
  (return))

(fn `SaveNewGoldScore`
  (params (SaveGameHS :type "/Game/UI/SaveGameHS Object Reference") (NewTopScore :type Integer))
  (`self.SaveNewBronzeScore` SaveGameHS (`/Game/UI/SaveGameHS.SilverScore` SaveGameHS))
  (`self.SaveNewSilverScore` SaveGameHS (`/Game/UI/SaveGameHS.GoldScore` SaveGameHS))
  (set `/Game/UI/SaveGameHS.GoldScore` NewTopScore SaveGameHS)
  (return))

(fn `SaveNewSilverScore`
  (params (SaveGameHs :type "/Game/UI/SaveGameHS Object Reference") (NewTopScore :type Integer))
  (`self.SaveNewBronzeScore` SaveGameHs (`/Game/UI/SaveGameHS.SilverScore` SaveGameHs))
  (set `/Game/UI/SaveGameHS.SilverScore` NewTopScore SaveGameHs)
  (return))

(fn `StopAllPlayerInput`
  (bind _outactors (`GameplayStatics.GetAllActorsOfClass` "/Game/Custom/BP_Player1.BP_Player1_C"))
  (for _array_element _outactors
    _))

(fn `TryStoreHighScore`
  (params (TopScore :type Integer))
  ;[0.1229 0.2293 1] Load Data
  (bind _output_get (set `self.SaveGameFileName` "SaveFile"))
  (bind _returnvalue (`KismetStringLibrary.Conv_NameToString` _output_get))
  (bind _returnvalue_2 (`GameplayStatics.DoesSaveGameExist` _returnvalue))
  (if _returnvalue_2
    (bind _returnvalue_3 (`GameplayStatics.LoadGameFromSlot` _returnvalue))
    (bind _assave_game_hs (cast `/Game/UI/SaveGameHS` _returnvalue_3))
    ;[1 0.807 0.1156] Gold Score
    (if (< (`/Game/UI/SaveGameHS.GoldScore` _assave_game_hs) TopScore)
      (`self.SaveNewGoldScore` _assave_game_hs TopScore)
      ;[0.2711 0.2828 1] SaveData
      (`GameplayStatics.SaveGameToSlot` _assave_game_hs (`KismetStringLibrary.Conv_NameToString` (`self.SaveGameFileName`)) :!label _label)
      (return)
      (else
        ;[1 1 1] Silver Text
        (if (< (`/Game/UI/SaveGameHS.SilverScore` _assave_game_hs) TopScore)
          (`self.SaveNewSilverScore` _assave_game_hs TopScore)
          (goto _label)
          (else
            ;[1 0.8186 0.3588] Bronze Text
            (if (< (`/Game/UI/SaveGameHS.BronzeScore` _assave_game_hs) TopScore)
              (`self.SaveNewBronzeScore` _assave_game_hs TopScore)
              (goto _label))))))))

(fn `UserConstructionScript`)