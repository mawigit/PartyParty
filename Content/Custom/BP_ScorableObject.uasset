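; BP_ScorableObject is a physics-simulated pickup actor that scores for the player when it reaches a TeleportZone.
; On begin play it enables physics and gravity on its body.
; When it overlaps a TeleportZone, it destroys itself, plays a sound, and asks the BP_ScorableObjectSpawner to spawn another.
; It then calls AddScore on player 0's BP_Player1 character.
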(event `self.ReceiveBeginPlay`
  (bind _scorableobjectbody (`self.ScorableObjectBody`))
  (`PrimitiveComponent.SetSimulatePhysics` _scorableobjectbody true)
  (`PrimitiveComponent.SetEnableGravity` _scorableobjectbody true))

(event `self.ReceiveActorBeginOverlap`
  (params (OtherActor :type "Actor Object Reference"))
  (cast `/Game/Custom/TeleportZone` OtherActor)
  (`self.K2_DestroyActor`)
  (`GameplayStatics.PlaySound2D` "/Game/SFX/345297__scrampunk__itemize.345297__scrampunk__itemize" 1.0 1.0 0.0 null null)
  (bind _returnvalue (`GameplayStatics.GetActorOfClass` "/Game/Custom/BP_ScorableObjectSpawner.BP_ScorableObjectSpawner_C"))
  (`/Game/Custom/BP_ScorableObjectSpawner.SpawnScorableObject` _returnvalue)
  (bind _asbp_player_1 (cast `/Game/Custom/BP_Player1` (`GameplayStatics.GetPlayerCharacter` 0)))
  (`/Game/Custom/BP_Player1.AddScore` _asbp_player_1))

(fn `UserConstructionScript`)