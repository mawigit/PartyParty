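; BP_ExplosiveObstacle is a mine-like obstacle that stuns and launches the player when its Hit event fires.
; Hit destroys the Sphere component, briefly stuns the BP_Player1 found by class lookup, and plays a 2D blast sound.
; A velocity-change impulse on the player's capsule pushes it away from the obstacle with a fixed upward boost.
; The actor itself remains, as its DestroyActor node is unconnected.
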(event `self.ReceiveHit`
  (params (MyComp :type "PrimitiveComponent Object Reference") (Other :type "Actor Object Reference") (OtherComp :type "PrimitiveComponent Object Reference") (bSelfMoved :type Boolean) (HitLocation :type "Vector Structure") (HitNormal :type "Vector Structure") (NormalImpulse :type "Vector Structure") (Hit :type "HitResult Structure (by ref)"))
  (`ActorComponent.K2_DestroyComponent` (`self.Sphere`))
  (bind _returnvalue (`GameplayStatics.GetActorOfClass` "/Game/Custom/BP_Player1.BP_Player1_C"))
  (`/Game/Custom/BP_Player1.Stun` _returnvalue 0.5)
  (`PrimitiveComponent.AddImpulse` (`Character.CapsuleComponent` _returnvalue) (`KismetMathLibrary.MakeVector` (.x (* (`KismetMathLibrary.GetDirectionUnitVector` (`self.K2_GetActorLocation`) (`self.K2_GetActorLocation` _returnvalue)) (`KismetMathLibrary.Conv_DoubleToVector` 2500.0))) (.y (* (`KismetMathLibrary.GetDirectionUnitVector` (`self.K2_GetActorLocation`) (`self.K2_GetActorLocation` _returnvalue)) (`KismetMathLibrary.Conv_DoubleToVector` 2500.0))) 1000.0) "None" true)
  (`GameplayStatics.PlaySound2D` "/Game/SFX/mine_blast.mine_blast" 1.5 1.0 0.0 null null false))

(fn `UserConstructionScript`
  (`parent.UserConstructionScript`))