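; BP_WaveObstacle is a moving obstacle that knocks the player away on contact.
; A Timeline started at BeginPlay drives the Y position of its elongated Cube through the UpDown track.
; Any actor overlap looks up BP_Player1 by class and briefly enables physics on its capsule to apply a velocity-change impulse along X, then disables physics after a short delay.
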(event `self.ReceiveBeginPlay`
  (bind _cube (`self.Cube`))
  (bind (_relativelocation_x _relativelocation_y _relativelocation_z) (`KismetMathLibrary.BreakVector` (`SceneComponent.RelativeLocation` _cube)))
  (bind (_direction _updown) (`Timeline|Timeline` :!via `PlayFromStart`)
    (:`Update`
      (`SceneComponent.K2_SetRelativeTransform` _cube (`KismetMathLibrary.MakeTransform` (`KismetMathLibrary.MakeVector` _relativelocation_x _updown _relativelocation_z) (struct :`Pitch` 90.0) (1.0 1.0 30.0)) false false))))

(event `self.ReceiveActorBeginOverlap`
  (params (OtherActor :type "Actor Object Reference"))
  (bind _returnvalue (`GameplayStatics.GetActorOfClass` "/Game/Custom/BP_Player1.BP_Player1_C"))
  (bind _capsulecomponent (`Character.CapsuleComponent` _returnvalue))
  (`PrimitiveComponent.SetSimulatePhysics` _capsulecomponent true)
  (`PrimitiveComponent.AddImpulse` _capsulecomponent (1000.0 0.0 0.0) "None" true)
  (`KismetSystemLibrary.Delay` 0.1)
  (`PrimitiveComponent.SetSimulatePhysics` _capsulecomponent false))

(fn `UserConstructionScript`)