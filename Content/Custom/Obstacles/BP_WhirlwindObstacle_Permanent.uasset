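; Permanent whirlwind obstacle that flings and spins the player upward when its Hit event runs.
; Hit finds BP_Player1 by class, briefly enables capsule physics for upward and yaw impulses, and plays a whoosh and fall animation.
; After a short delay it restores the Animation Blueprint and turns physics off.
; The file does not show what triggers Hit; construction only calls the parent.
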(event `self.ReceiveHit`
  (params (MyComp :type "PrimitiveComponent Object Reference") (Other :type "Actor Object Reference") (OtherComp :type "PrimitiveComponent Object Reference") (bSelfMoved :type Boolean) (HitLocation :type "Vector Structure") (HitNormal :type "Vector Structure") (NormalImpulse :type "Vector Structure") (Hit :type "HitResult Structure (by ref)"))
  (bind _returnvalue (`GameplayStatics.GetActorOfClass` "/Game/Custom/BP_Player1.BP_Player1_C"))
  (bind _capsulecomponent (`Character.CapsuleComponent` _returnvalue))
  (`PrimitiveComponent.SetSimulatePhysics` _capsulecomponent true)
  (`GameplayStatics.PlaySound2D` "/Game/SFX/60028__qubodup__double-whoosh.60028__qubodup__double-whoosh" 1.0 1.0 0.0 null null)
  (`PrimitiveComponent.AddAngularImpulseInDegrees` _capsulecomponent (0.0 0.0 10000.0) "None" true)
  (`PrimitiveComponent.AddImpulse` _capsulecomponent (0.0 0.0 1000.0) "None" true)
  (bind _mesh (`Character.Mesh` _returnvalue))
  (`SkeletalMeshComponent.PlayAnimation` _mesh "/Game/ThirdParty/LUSH_StylizedEnvironmentSet/EpicDemoContent/Characters/Mannequins/Animations/Manny/A_Demo_MM_Fall_Loop.A_Demo_MM_Fall_Loop" false)
  (`KismetSystemLibrary.Delay` 0.5)
  (`SkeletalMeshComponent.SetAnimationMode` _mesh "AnimationBlueprint" true)
  (`PrimitiveComponent.SetSimulatePhysics` _capsulecomponent false))

(fn `UserConstructionScript`
  (`parent.UserConstructionScript`))